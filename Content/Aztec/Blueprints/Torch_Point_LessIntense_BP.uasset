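; Torch point light Blueprint that flickers its light's intensity and shifts it vertically.
; A random delay on BeginPlay offsets the start of the Flickering timeline, whose curve drives intensity with a random multiplier on each update.
; Each Flickering update also re-captures the light's world position and calls Play on the Move timeline, which adds its curve value to that position's Z.
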(event `self.ReceiveBeginPlay`
  (bind _pointlight (`self.PointLight`))
  (bind (_initpos_x _initpos_y _initpos_z) (`KismetMathLibrary.BreakVector` (`self.InitPos`)))
  (`KismetSystemLibrary.Delay` (`KismetMathLibrary.RandomFloatInRange` 0.0 0.8))
  (bind (_direction _intensity) (`Timeline|flickering`)
    (:`Update`
      (`LightComponent.SetIntensity` (`self.PointLight`) (* (* _intensity 2000.0) (`KismetMathLibrary.RandomFloatInRange` 1.0 1.5)))
      (set `self.InitPos` (`SceneComponent.K2_GetComponentLocation` _pointlight))
      (bind (_direction_2 _intensity_2) (`Timeline|Move`)
        (:`Update`
          (`SceneComponent.K2_SetWorldLocation` _pointlight (`KismetMathLibrary.MakeVector` _initpos_x _initpos_y (+ _intensity_2 _initpos_z)) false false))))))

(fn `UserConstructionScript`)