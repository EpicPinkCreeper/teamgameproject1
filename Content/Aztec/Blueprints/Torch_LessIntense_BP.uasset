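; Torch Blueprint for the Aztec content that animates a flickering spot light, named as a less intense variant.
; After a short random start delay, the Flickering timeline drives light intensity with a random multiplier on each update.
; Each flicker update also stores the light's current world location and calls Play on a second timeline, which offsets the light's height from that stored position.
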(event `self.ReceiveBeginPlay`
  (bind _spotlight (`self.SpotLight`))
  (bind (_initpos_x _initpos_y _initpos_z) (`KismetMathLibrary.BreakVector` (`self.InitPos`)))
  (`KismetSystemLibrary.Delay` (`KismetMathLibrary.RandomFloatInRange` 0.0 0.8))
  (bind (_direction _intensity) (`Timeline|flickering`)
    (:`Update`
      (`LightComponent.SetIntensity` _spotlight (* (* _intensity 100.0) (`KismetMathLibrary.RandomFloatInRange` 1.0 1.5)))
      (set `self.InitPos` (`SceneComponent.K2_GetComponentLocation` _spotlight))
      (bind (_direction_2 _intensity_2) (`Timeline|Timeline_0`)
        (:`Update`
          (`SceneComponent.K2_SetWorldLocation` _spotlight (`KismetMathLibrary.MakeVector` _initpos_x _initpos_y (+ _intensity_2 _initpos_z)) false false))))))

(fn `UserConstructionScript`)