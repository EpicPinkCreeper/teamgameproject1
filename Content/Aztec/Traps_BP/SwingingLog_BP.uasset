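; Swinging log trap Blueprint that rotates its beam mesh back and forth in the level.
; On BeginPlay it stores the mesh's starting world rotation, waits a random delay, then plays a timeline whose track adds an offset to roll while keeping pitch and yaw.
; When the timeline finishes, it restarts from the start after a short random pause, so placed instances swing out of sync.
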(event `self.ReceiveBeginPlay`
  (bind (_initrot_roll _initrot_pitch _initrot_yaw) (`KismetMathLibrary.BreakRotator` (`self.InitRot`)))
  (set `self.InitRot` (`SceneComponent.K2_GetComponentRotation` (`self.A_SwingingBeam_V1_Geo`)))
  (`KismetSystemLibrary.Delay` (`KismetMathLibrary.RandomFloatInRange` 0.0 2.0))
  (bind (_direction _newtrack) (`Timeline|Timeline_0` :!label _label)
    (:`Update`
      (`SceneComponent.K2_SetWorldRotation` (`self.A_SwingingBeam_V1_Geo`) (`KismetMathLibrary.MakeRotator` (+ _newtrack _initrot_roll) _initrot_pitch _initrot_yaw) false false))
    (:`Finished`
      (`KismetSystemLibrary.Delay` (`KismetMathLibrary.RandomFloatInRange` 0.0 0.2))
      (goto _label :!via `PlayFromStart`))))

(fn `UserConstructionScript`)